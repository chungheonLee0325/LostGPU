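; Game state for the Saydon boss fight, driving phase progression and the recurring hammer attack.
; BeginPlay shows the boss HUD and attaches a crosshair above the player.
; Until phase four, Tick times Saydon's strikes, debug-draws a circle at the player and briefly hides the crosshair.
; NextPhase spawns cards with one random Joker, later swaps them for Kakul, then triggers victory; a helper tests card-in-circle containment.
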(event `self.ReceiveBeginPlay`
  (bind _returnvalue (`GameplayStatics.GetActorOfClass` "/Game/_BluePrint/Common/BP_Character.BP_Character_C"))
  (bind _output_get (set `self.Player` _returnvalue))
  (bind _asbp_character (cast `/Game/_BluePrint/Common/BP_Character` _output_get))
  (`/Game/_BluePrint/Common/Widget/HUD_Boss.Set_BossHUD_Visibility` (`/Game/_BluePrint/Common/Widget/HUD.HUD_BossHP` (`/Game/_BluePrint/Common/BP_Character.HUD Reference` _asbp_character)) "Visible")
  (bind _returnvalue_2 (`GameplayStatics.GetActorOfClass` "/Game/_BluePrint/KBD/BP_Saydon.BP_Saydon_C"))
  (set `self.Saydon` _returnvalue_2)
  (bind _returnvalue_3 (`GameplayStatics.GetActorOfClass` "/Game/_BluePrint/KBD/BP_Kakul.BP_Kakul_C"))
  (set `self.Kakul` _returnvalue_3)
  ; 플레이어 머리 위에 과녁을 표시
  (bind _returnvalue_4 (`AddComponent|NODE_AddWidgetComponent-0` :`self` (`self.Player`) :`RelativeTransform` (`KismetMathLibrary.MakeTransform` (0.0 0.0 200.0) (struct :`Yaw` 90.0))))
  (set `self.CrosshairWidget` (`WidgetComponent.GetUserWidgetObject` _returnvalue_4)))

(event `self.ReceiveTick`
  (params (DeltaSeconds :type "Float (single-precision)"))
  (bind _crosshairwidget (`self.CrosshairWidget`))
  (bind (_returnvalue_x _returnvalue_y) (`KismetMathLibrary.BreakVector` (`self.K2_GetActorLocation` (`self.Player`))))
  (if (< (`self.CurrentPhase`) 4)
    (set `self.CurrentTime` (+ DeltaSeconds (`self.CurrentTime`)))
    (`/Engine/EditorBlueprintResources/StandardMacros.IsValid` (`self.Player`)
      (:`Is Valid`
        ; 망치를 내려쳐야 할 시간이 되었으면
        (if (>= (`self.CurrentTime`) (`self.Hummer Time`))
          ; 범위 디버깅
          (`KismetSystemLibrary.DrawDebugCircle` (`KismetMathLibrary.MakeVector` _returnvalue_x _returnvalue_y 10.0) 0.0 64 (struct :`R` 1.0 :`A` 1.0) 2.5 3.0 (1.0 0.0 0.0) (0.0 1.0 0.0))
          (`/Game/_BluePrint/KBD/BP_Saydon.StrikeHammer` (`self.Saydon`))
          (set `self.CurrentTime` 0.0)
          (`/Engine/EditorBlueprintResources/StandardMacros.IsValid` _crosshairwidget
            (:`Is Valid`
              (`Widget.SetRenderOpacity` _crosshairwidget 0.0)
              (`KismetSystemLibrary.Delay` 1.3)
              (`Widget.SetRenderOpacity` _crosshairwidget 1.0)))))
      (:`Is Not Valid`
        (`KismetSystemLibrary.PrintString` "Player Is None")))))

(event `NextPhase`
  (bind _result (`/Engine/EditorBlueprintResources/StandardMacros.IncrementInt` (`self.CurrentPhase`))
    (:`  `
      (bind _output_get (set `self.CurrentPhase` _result))
      (switch `int` _output_get
        (:`Default`
          ; 4페이즈는 없고 게임 클리어
          (bind _asbp_character (cast `/Game/_BluePrint/Common/BP_Character` (`self.Player`)))
          (`/Game/_BluePrint/Common/Widget/HUD.GameWin` (`/Game/_BluePrint/Common/BP_Character.HUD Reference` _asbp_character))
          (`SceneComponent.SetVisibility` (`/Game/_BluePrint/KBD/BP_Saydon.Saydon_v1` (`self.Saydon`)) false true))
        (:`2`
          ; 2페이즈 - 세이튼 카드 패턴 시작
          (`self.SpawnCard`))
        (:`3`
          ; 3페이즈 - 카드 제거 후 쿠크 재등장
          (bind _outactors (`GameplayStatics.GetAllActorsOfClass` "/Game/_BluePrint/KBD/BP_Card.BP_Card_C"))
          (for _array_element _outactors
            (`self.K2_DestroyActor` _array_element))
          (`|SpawnActorFromClass` "/Game/_BluePrint/KBD/BP_Kakul.BP_Kakul_C" (`KismetMathLibrary.MakeTransform` (400.0 0.0 0.0) (struct :`Yaw` 179.9)) "Undefined" "MultiplyWithRoot" null null))))))

(event `SpawnCard`
  ; 카드 소환
  (bind _returnvalue (`KismetMathLibrary.RandomIntegerInRange` 0 6))
  (bind _outactors (`GameplayStatics.GetAllActorsOfClass` "/Game/_BluePrint/KBD/BP_CardSpawnPoint.BP_CardSpawnPoint_C"))
  (for (_array_element _array_index) _outactors
    (bind _returnvalue_2 (`|SpawnActorFromClass` "/Game/_BluePrint/KBD/BP_Card.BP_Card_C" (`KismetMathLibrary.MakeTransform` (`self.K2_GetActorLocation` _array_element)) "Undefined" "MultiplyWithRoot" null null))
    (if (== _array_index _returnvalue)
      (bind _output_get (set `self.JokerCard` _returnvalue_2))
      (set `/Game/_BluePrint/KBD/BP_Card.IsJoker` true _returnvalue_2)
      (`PrimitiveComponent.SetMaterial` (`/Game/_BluePrint/KBD/BP_Card.Body` _output_get) 0 "/Game/_Resource/Character/Boss/Saydon/Card/Joker.Joker")))
  (set `self.SaydonState` "NewEnumerator1"))

(fn `IsCardContainInCircle`
  (params (cardCenterLocation :type "Vector Structure") (`cardWidth/2` :type "Float (double-precision)") (`cardHeight/2` :type "Float (double-precision)") (circleCenterLocation :type "Vector Structure") (circleRadius :type "Float (double-precision)") (cardCenterLocation_X :type "Float (double-precision)" :default 0.0) (cardCenterLocation_Y :type "Float (double-precision)" :default 0.0) (cardCenterLocation_Z :type "Float (double-precision)" :default 0.0) (circleCenterLocation_X :type "Float (double-precision)" :default 0.0) (circleCenterLocation_Y :type "Float (double-precision)" :default 0.0) (circleCenterLocation_Z :type "Float (double-precision)" :default 0.0))
  (returns (IsContain :type Boolean))
  (return (and (and (<= (`KismetMathLibrary.Abs` (- (+ cardCenterLocation_X `cardWidth/2`) circleCenterLocation_X)) circleRadius) (<= (`KismetMathLibrary.Abs` (- (- cardCenterLocation_X `cardWidth/2`) circleCenterLocation_X)) circleRadius)) (and (<= (`KismetMathLibrary.Abs` (- (+ cardCenterLocation_Y `cardHeight/2`) circleCenterLocation_Y)) circleRadius) (<= (`KismetMathLibrary.Abs` (- (- cardCenterLocation_Y `cardHeight/2`) circleCenterLocation_Y)) circleRadius)))))

(fn `UserConstructionScript`)