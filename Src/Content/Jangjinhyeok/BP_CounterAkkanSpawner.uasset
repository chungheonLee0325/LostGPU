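; Spawner actor that periodically creates BP_CounterAkkan actors on a ring around itself.
; Tick accumulates time and, once it exceeds CreateTime, resets it and spawns one at a random angle on the circle defined by the SpawnArea sphere's scaled radius.
; Each spawn sits at the spawner's height and is rotated to face the center.
; BeginPlay reuses the same spawn logic to create one immediately for testing.
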(event `self.ReceiveTick`
  (params (DeltaSeconds :type "Float (single-precision)"))
  ; 시간이 흐른다
  (set `self.CurrentTime` (+ (`self.CurrentTime`) DeltaSeconds))
  ; 생성시간을 초과했다면
  (if (> (`self.CurrentTime`) (`self.CreateTime`))
    ; 경과시간 초기화
    (set `self.CurrentTime` 0.0)
    ; 0~360의 랜덤한 각도를 생성 후 radian으로 변경
    (bind _output_get (set `self.RandomAngle` (* (`KismetMathLibrary.RandomFloatInRange` 0.0 1.0) (`self.Angle`)) :!label _label))
    (bind _output_get_2 (set `self.RandomRadian` (`KismetMathLibrary.DegreesToRadians` _output_get)))
    ; x,y 좌표 계산 후 Random Location 설정 후 현재 위치와 합침
    ;; x = cosΘ * radius
    (bind _output_get_3 (set `self.RandomX` (* (`KismetMathLibrary.Cos` _output_get_2) (`SphereComponent.GetScaledSphereRadius` (`self.SpawnArea`)))))
    ;; y = sinΘ * radius
    (bind _output_get_4 (set `self.RandomY` (* (`KismetMathLibrary.Sin` _output_get_2) (`SphereComponent.GetScaledSphereRadius` (`self.SpawnArea`)))))
    (bind _output_get_5 (set `self.RandomLoc` (`KismetMathLibrary.MakeVector` _output_get_3 _output_get_4)))
    (bind _returnvalue (+ _output_get_5 (`self.K2_GetActorLocation`)))
    (`|SpawnActorFromClass` "/Game/Jangjinhyeok/BP_CounterAkkan.BP_CounterAkkan_C" (`KismetMathLibrary.MakeTransform` _returnvalue (`KismetMathLibrary.FindLookAtRotation` _returnvalue (`self.K2_GetActorLocation`))) "Undefined" "MultiplyWithRoot" null null)))

(event `self.ReceiveBeginPlay`
  ; 테스트용으로 시작하자마자 한 개 생성
  (goto _label))

(fn `UserConstructionScript`)