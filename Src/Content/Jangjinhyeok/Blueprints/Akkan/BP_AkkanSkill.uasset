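; BP_AkkanSkill is the telegraph actor for an Akkan laser attack, showing a fan-shaped range that widens while tracking the player.
; Until TrackingTime elapses, Tick plays the GettingBigger timeline, which drives Y scale and yaws the actor toward the player with pitch fixed at 90.
; It then spawns BP_AkkanAttack at its location, aimed at the player's current position, and destroys itself.
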(event `self.ReceiveTick`
  (params (DeltaSeconds :type "Float (single-precision)"))
  (bind (_returnvalue_x _returnvalue_y _returnvalue_z) (`KismetMathLibrary.BreakVector` (`self.GetActorScale3D`)))
  (bind _returnvalue (`self.K2_GetActorLocation`))
  (bind _returnvalue_2 (`self.K2_GetActorLocation` (`GameplayStatics.GetPlayerPawn` 0)))
  (bind (_returnvalue_roll _returnvalue_pitch _returnvalue_yaw) (`KismetMathLibrary.BreakRotator` (`KismetMathLibrary.FindLookAtRotation` _returnvalue _returnvalue_2)))
  ; 경과시간이 추적시간 보다 작다면
  (bind _output_get (set `self.CurrentTime` (+ DeltaSeconds (`self.CurrentTime`))))
  (if (< _output_get (`self.TrackingTime`))
    ; 플레이어를 추적하는 부채꼴 범위가 점점 확장됨
    (bind (_direction _size) (`Timeline|Getting Bigger` :`NewTime` DeltaSeconds)
      (:`Update`
        (`self.SetActorScale3D` (`KismetMathLibrary.MakeVector` _returnvalue_x _size _returnvalue_z))
        (set `self.LookAtVector` (- _returnvalue_2 _returnvalue))
        (`self.K2_SetActorRotation` (`KismetMathLibrary.MakeRotator` _returnvalue_roll 90.0 _returnvalue_yaw))))
    (else
      ; 레이저 공격 BP소환
      (`|SpawnActorFromClass` "/Game/Jangjinhyeok/Blueprints/Akkan/BP_AkkanAttack.BP_AkkanAttack_C" (`KismetMathLibrary.MakeTransform` (`self.K2_GetActorLocation`) (`KismetMathLibrary.FindLookAtRotation` _returnvalue _returnvalue_2)) "Undefined" "MultiplyWithRoot" null null)
      (`self.K2_DestroyActor`))))

(fn `UserConstructionScript`)