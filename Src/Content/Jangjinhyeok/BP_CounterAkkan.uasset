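; BP_CounterAkkan is an actor that runs a timed counter sequence followed by forward movement.
; Tick accumulates elapsed time and, once past CounterStartTime, prints "Do Counter!" every frame as a placeholder for a future effect.
; Once time also passes MoveStartTime, it moves at Speed along the constant world forward vector, scaled by delta time, without sweep.
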(event `self.ReceiveTick`
  (params (DeltaSeconds :type "Float (single-precision)"))
  ; 시간이 흐른다
  (bind _output_get (set `self.CurrentTime` (+ DeltaSeconds (`self.CurrentTime`))))
  ; 카운터 칠 시간이 지나면
  (if (> _output_get (`self.CounterStartTime`))
    ; 이펙트로 변경할 부분
    (`KismetSystemLibrary.PrintString` "Do Counter!")
    ; 움직일 수 있는 시간이 되면
    (if (> (`self.CurrentTime`) (`self.MoveStartTime`))
      ; 앞으로 가라
      (`self.K2_SetActorLocation` (+ (* DeltaSeconds (* (`self.Speed`) (`KismetMathLibrary.Vector_Forward`))) (`self.K2_GetActorLocation`))))))

(fn `UserConstructionScript`)