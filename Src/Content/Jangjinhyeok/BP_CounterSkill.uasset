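; BP_CounterSkill is a short-lived counter skill actor that flags a BP_CounterAkkan as hit by a counter when it overlaps one.
; On overlap it sets IsHittedCounter on the first actor found by GetActorOfClass for that class, not directly on the overlapped actor, and prints the flag.
; Tick accumulates elapsed time and destroys the actor after a fraction of a second.
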(event `self.ReceiveActorBeginOverlap`
  (params (OtherActor :type "Actor Object Reference"))
  (bind _asbp_counter_akkan (cast `/Game/Jangjinhyeok/Akkan/BP_CounterAkkan` OtherActor))
  (bind _returnvalue (`GameplayStatics.GetActorOfClass` (`GameplayStatics.GetObjectClass` _asbp_counter_akkan)))
  (bind _output_get (set `/Game/Jangjinhyeok/Akkan/BP_CounterAkkan.IsHittedCounter` true _returnvalue))
  (`KismetSystemLibrary.PrintString` (`KismetStringLibrary.Conv_BoolToString` _output_get)))

(event `self.ReceiveTick`
  (params (DeltaSeconds :type "Float (single-precision)"))
  (bind _output_get (set `self.CurrentTime` (+ DeltaSeconds (`self.CurrentTime`))))
  (if (> _output_get 0.7)
    (`self.K2_DestroyActor`)))

(fn `UserConstructionScript`)