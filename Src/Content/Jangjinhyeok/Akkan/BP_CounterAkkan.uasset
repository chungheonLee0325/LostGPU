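; BP_CounterAkkan is a spawned Akkan (Illiakan) actor for a counter pattern, removed when countered or when its time runs out.
; Tick accumulates elapsed time and, once both the counter-start and move-start thresholds pass, calls MoveForward until DestroyTime triggers destruction.
; MoveForward offsets location along the forward vector by Speed and delta time, without sweeping.
; IsHittedCounter, not set in this graph, destroys it immediately when true.
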(event `self.ReceiveTick`
  (params (DeltaSeconds :type "Float (single-precision)"))
  ; 시간이 흐른다
  (bind _output_get (set `self.CurrentTime` (+ DeltaSeconds (`self.CurrentTime`))))
  ; 카운터 성공 시 obj삭제
  (if (`self.IsHittedCounter`)
    ; 스폰된 카운터 일리아칸 삭제 시간 설정
    (`self.K2_DestroyActor` :!label _label)
    (else
      ; 카운터 칠 시간이 지나고
      (if (> _output_get (`self.CounterStartTime`))
        ; 움직일 수 있는 시간이 되면
        (if (> (`self.CurrentTime`) (`self.MoveStartTime`))
          (`self.MoveForward` DeltaSeconds)
          (if (> (`self.CurrentTime`) (`self.DestroyTime`))
            (goto _label)))))))

(fn `MoveForward`
  (params (DeltaTime :type "Float (single-precision)"))
  ; 앞으로 가라
  (`self.K2_SetActorLocation` (+ (* DeltaTime (* (`self.Speed`) (`self.GetActorForwardVector`))) (`self.K2_GetActorLocation`))))

(fn `UserConstructionScript`)