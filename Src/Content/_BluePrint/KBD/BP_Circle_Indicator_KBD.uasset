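; BP_Circle_Indicator_KBD is a timed circle indicator actor that animates its size and then destroys itself.
; InitializeCI sets its lifetime, hit time and overall actor scale.
; Each Tick plays CircleSizeTimeLine at a rate of one over HitTime, so the circle's scale animation follows the hit timing.
; Timeline updates scale the Circle component and also count down LifeTime, destroying the actor when it runs out.
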(event `self.ReceiveTick`
  (params (DeltaSeconds :type "Float (single-precision)"))
  (`TimelineComponent.SetPlayRate` (`self.CircleSizeTimeLine`) (/ 1.0 (`self.hitTime`)))
  (bind (_direction _size) (`Timeline|CircleSizeTimeLine` :`NewTime` DeltaSeconds)
    (:`Update`
      (`SceneComponent.SetRelativeScale3D` (`self.Circle`) (* (`KismetMathLibrary.Vector_One`) _size))
      (bind _output_get (set `self.lifeTime` (- (`self.lifeTime`) DeltaSeconds)))
      (if (<= _output_get 0.0)
        (`self.K2_DestroyActor`)))))

(event `InitializeCI`
  (params (lifeTime :type "Float (double-precision)") (hitTime :type "Float (double-precision)") (Scale :type "Float (double-precision)"))
  (set `self.lifeTime` lifeTime)
  (set `self.hitTime` hitTime)
  (`self.SetActorScale3D` (`KismetMathLibrary.Conv_DoubleToVector` Scale)))

(fn `UserConstructionScript`)