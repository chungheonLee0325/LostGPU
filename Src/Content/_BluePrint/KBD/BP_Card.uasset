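; BP_Card is a card actor that animates a peek or full flip and can advance the game phase.
; A half flip drives height and pitch through a timeline, which reverses on finish when IsFlipping is set.
; A full flip animates height and rotation, marking the card flipped to block further flips.
; A three-second Delay from the flip's Update destroys the card, first calling NextPhase on BP_SaydonGameState for Jokers.
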(event `self.ReceiveTick`
  (params (DeltaSeconds :type "Float (single-precision)")))

(event `PlayCardFlip`
  (params (IsFullFlip :type Boolean))
  (bind _returnvalue (`self.GetTransform`))
  (if (`self.IsFlipped`)
    _
    (elif IsFullFlip
      (bind (_direction _locationz _rotationy _rotationx _rotationz) (`Timeline|FullFlip`)
        (:`Update`
          (`self.K2_SetActorTransform` (`KismetMathLibrary.MakeTransform` (`KismetMathLibrary.MakeVector` (.x (.location _returnvalue)) (.y (.location _returnvalue)) _locationz) (`KismetMathLibrary.MakeRotator` _rotationx _rotationy _rotationz)))
          (`KismetSystemLibrary.Delay` 3.0)
          (if (`self.IsJoker`)
            (bind _asbp_saydon_game_state (cast `/Game/_Maps/Saydon/BP_SaydonGameState` (`GameplayStatics.GetGameState`)))
            (`/Game/_Maps/Saydon/BP_SaydonGameState.NextPhase` _asbp_saydon_game_state))
          (`self.K2_DestroyActor`))
        (:`Finished`
          (set `self.IsFlipped` true)))
      (else
        (bind (_direction_2 _locationz_2 _rotationy_2) (`Timeline|HalfFlip` :!label _label)
          (:`Update`
            (`self.K2_SetActorTransform` (`KismetMathLibrary.MakeTransform` (`KismetMathLibrary.MakeVector` (.x (.location _returnvalue)) (.y (.location _returnvalue)) _locationz_2) (`KismetMathLibrary.MakeRotator` (.roll (.rotation _returnvalue)) _rotationy_2 (.yaw (.rotation _returnvalue))) (.scale _returnvalue))))
          (:`Finished`
            ; 카드를 다 띄우고 나면 다시 원래 자리로 놓아라
            (if (`self.IsFlipping`)
              (`self.ReverseCardFlip`)
              (set `self.IsFlipping` false))))))))

(event `ReverseCardFlip`
  (goto _label :!via `Reverse`))

(fn `UserConstructionScript`)