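; Blueprint function library with a single geometry helper, IsRectInCircle, that tests whether a rectangle lies within a circle.
; It offsets the rectangle's location by its half width and half height, then compares each edge's X or Y distance from the circle center to the radius.
; Axes are checked independently, so it effectively tests containment in the circle's bounding square, and corners can fall outside the actual circle.
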(fn `IsRectInCircle`
  (params (RectLocation :type "Vector Structure") (`RectWidth/2` :type "Float (double-precision)") (`RectHeight/2` :type "Float (double-precision)") (CircleLocation :type "Vector Structure") (CircleRadius :type "Float (double-precision)"))
  (returns (IsContain :type Boolean))
  (return (and (and (<= (`KismetMathLibrary.Abs` (- (+ RectLocation_X `RectWidth/2`) CircleLocation_X)) CircleRadius) (<= (`KismetMathLibrary.Abs` (- (- RectLocation_X `RectWidth/2`) CircleLocation_X)) CircleRadius)) (and (<= (`KismetMathLibrary.Abs` (- (+ RectLocation_Y `RectHeight/2`) CircleLocation_Y)) CircleRadius) (<= (`KismetMathLibrary.Abs` (- (- RectLocation_Y `RectHeight/2`) CircleLocation_Y)) CircleRadius)))))