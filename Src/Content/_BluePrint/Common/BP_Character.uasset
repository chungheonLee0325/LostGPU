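; Player character Blueprint that sets up the HUD and handles death.
; BeginPlay calls the parent, adds the HUD to the viewport and creates dynamic instances of both Manny mesh materials.
; OnDie prints a placeholder for animation, fade-out and UI, then destroys the actor after a delay; OnKill, OnRevival and Hit (marked for deletion) are empty.
; Disconnected leftover nodes hold Circle_Indicator test spawns and status-effect hit reactions using montages and Tint flashes.
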(event `self.ReceiveBeginPlay`
  (bind _mesh (`self.Mesh`))
  (`parent.ReceiveBeginPlay`)
  ; HUD 출력
  (bind _returnvalue (`|CreateWidget` "/Game/_BluePrint/Common/Widget/HUD.HUD_C"))
  (bind _output_get (set `self.HUD Reference` _returnvalue))
  (`UserWidget.AddToViewport` _output_get 0)
  ; Material의 Parameter를 동적으로 변경하기 위해 Instance를 생성하고 Set
  (`|ExecutionSequence`
    (:`then_0`
      (bind _returnvalue_2 (`PrimitiveComponent.CreateDynamicMaterialInstance` _mesh 0 "/Game/Characters/Mannequins/Materials/Instances/Manny/MI_Manny_01.MI_Manny_01" "None"))
      (set `self.Material_0` _returnvalue_2))
    (:`then_1`
      (bind _returnvalue_3 (`PrimitiveComponent.CreateDynamicMaterialInstance` _mesh 1 "/Game/Characters/Mannequins/Materials/Instances/Manny/MI_Manny_02.MI_Manny_02" "None"))
      (set `self.Material_1` _returnvalue_3))))

(event `self.OnDie`
  (`KismetSystemLibrary.PrintString` "애니메이션 추가, 페이드아웃 이펙트, UI ")
  (`KismetSystemLibrary.Delay` 2.0)
  (`self.K2_DestroyActor`))

(event `self.OnKill`)

(event `self.OnRevival`)

(event `Hit`
  (params (statusEffectType :type "/Game/_BluePrint/Common/Enum/StatusEffectType Enum" :default "NewEnumerator1"))
  ;[0.15 0 0.0686 0.5] ToDo -> 삭제
)

(event `Key|Z`
  (params (Key :type "Key Structure"))
  ; Debug
)

(event `Key|X`
  (params (Key :type "Key Structure"))
  ; Debug
)

(event `Key|C`
  (params (Key :type "Key Structure"))
  ; Debug
)

(fn `UserConstructionScript`)