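; BP_DamageFloator is an actor Blueprint that displays combat feedback text on screen through the BP_Damage widget.
; FloatDamage creates a new widget per call, showing the amount for Damage and Critical Damage, or the type name for Knockdown, Stun and Destroy.
; Each widget is added to the viewport at the screen origin; the Target's location is not used, so the text does not follow the target.
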(fn `FloatDamage`
  (params (Type :type "/Game/_BluePrint/Common/Widget/DamageType Enum" :default "NewEnumerator0") (Amount :type "Float (double-precision)") (Target :type "Actor Object Reference"))
  (bind _returnvalue (`|CreateWidget` "/Game/_BluePrint/Common/Widget/BP_Damage.BP_Damage_C"))
  (switch `/Game/_BluePrint/Common/Widget/DamageType` Type
    (:`NewEnumerator0`
      (bind _output_get (set `self.DmgStr` (`KismetTextLibrary.Conv_DoubleToText` Amount "HalfToEven") :!label _label))
      (bind _damage (`/Game/_BluePrint/Common/Widget/BP_Damage.Damage` _returnvalue))
      (`TextBlock.SetText` _damage _output_get))
    (:`NewEnumerator1`
      (goto _label))
    (:`NewEnumerator2`
      (bind _output_get_2 (set `self.DmgStr` (`KismetTextLibrary.Conv_StringToText` (`|GetEnumeratorNameAsString` Type)) :!label _label_2))
      (`TextBlock.SetText` _damage _output_get_2))
    (:`NewEnumerator3`
      (goto _label_2))
    (:`NewEnumerator4`
      (goto _label_2)))
  (`UserWidget.AddToViewport` _returnvalue 0)
  (`UserWidget.SetPositionInViewport` _returnvalue (0.0 0.0) true))

(fn `UserConstructionScript`)