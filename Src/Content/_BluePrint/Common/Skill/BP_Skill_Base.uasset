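; BP_Skill_Base is a base Blueprint for skills that gates casting behind a cooldown.
; OnSkillCast returns the result of AdjustCoolTIme, which fails while on cooldown, or otherwise locks casting and starts a looping timer.
; CalcCoolTime counts the remaining cooldown down in tenth-second steps, then re-enables casting and clears the timer.
; On_Skill_Fire and On_Skill_Cancel are empty events, and nothing here calls them.
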(event `On_Skill_Fire`)

(event `On_Skill_Cancel`)

(fn `AdjustCoolTIme`
  (returns (skillCastSuccess :type Boolean))
  (if (`self.canCastSkill`)
    (set `self.canCastSkill` false)
    (set `self.currentCoolTime` (`self.CoolTime`))
    (bind _returnvalue (`KismetSystemLibrary.K2_SetTimer` null "CalcCoolTime" 0.1 true))
    (set `self.CalcCoolTimeHandle` _returnvalue)
    (return true)
    (else
      (return false))))

(fn `CalcCoolTime`
  (bind _output_get (set `self.currentCoolTime` (- (`self.currentCoolTime`) 0.1)))
  (bind _returnvalue (<= _output_get 0.0))
  (if _returnvalue
    (set `self.canCastSkill` _returnvalue)
    (`KismetSystemLibrary.K2_ClearAndInvalidateTimerHandle` (`self.CalcCoolTimeHandle`))))

(fn `On_Skill_Cast`
  (returns (Success :type Boolean))
  (bind _skillcastsuccess (`self.AdjustCoolTIme`))
  (return _skillcastsuccess))