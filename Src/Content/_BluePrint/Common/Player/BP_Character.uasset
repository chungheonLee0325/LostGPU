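; Player character Blueprint that gives hit feedback for damage, stun, knockback and knockdown, and destroys itself shortly after death.
; BeginPlay creates dynamic materials for two mesh slots, whose Tint StatusEffect briefly flashes per effect type, alongside montages for all but knockback.
; AnyDamage forwards damage to OnTakeDamage and reuses the damage reaction, while CanKnockDown blocks repeat knockdowns until the montage completes.
; Kill and revival events are empty, and debug Circle_Indicator spawns are disconnected.
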(event `self.ReceiveBeginPlay`
  (bind _mesh (`self.Mesh`))
  (`parent.ReceiveBeginPlay`)
  ; Material의 Parameter를 동적으로 변경하기 위해 Instance를 생성하고 Set
  (`|ExecutionSequence`
    (:`then_0`
      (bind _returnvalue (`PrimitiveComponent.CreateDynamicMaterialInstance` _mesh 0 "/Game/Characters/Mannequins/Materials/Instances/Manny/MI_Manny_01.MI_Manny_01" "None"))
      (set `self.Material_0` _returnvalue))
    (:`then_1`
      (bind _returnvalue_2 (`PrimitiveComponent.CreateDynamicMaterialInstance` _mesh 1 "/Game/Characters/Mannequins/Materials/Instances/Manny/MI_Manny_02.MI_Manny_02" "None"))
      (set `self.Material_1` _returnvalue_2))))

(event `StatusEffect`
  (params (statusEffectType :type "/Game/_BluePrint/Common/Enum/StatusEffectType Enum" :default "NewEnumerator1"))
  (switch `/Game/_BluePrint/Common/Enum/StatusEffectType` statusEffectType
    (:`NewEnumerator1`
      (`KismetSystemLibrary.PrintString` "Player_Hit" :!label _label)
      (`|PlayMontage` (`self.Mesh`) "/Game/_Resource/Character/Player/Animation/dmg_idle_1_Montage.dmg_idle_1_Montage"
        (:`then`
          ; 캐릭터를 빨간색으로 깜빡이게 한다
          (`|ExecutionSequence`
            (:`then_0`
              (`MaterialInstanceDynamic.SetVectorParameterValue` (`self.Material_0`) "Tint" (struct :`R` 1.0 :`A` 1.0)))
            (:`then_1`
              (`MaterialInstanceDynamic.SetVectorParameterValue` (`self.Material_1`) "Tint" (struct :`R` 1.0 :`A` 1.0))))
          (`KismetSystemLibrary.Delay` 0.15)
          (`|ExecutionSequence`
            (:`then_0`
              (`MaterialInstanceDynamic.SetVectorParameterValue` (`self.Material_0`) "Tint" (struct :`R` 1.0 :`G` 1.0 :`B` 1.0 :`A` 1.0)))
            (:`then_1`
              (`MaterialInstanceDynamic.SetVectorParameterValue` (`self.Material_1`) "Tint" (struct :`R` 1.0 :`G` 1.0 :`B` 1.0 :`A` 1.0)))))))
    (:`NewEnumerator0`
      (`KismetSystemLibrary.PrintString` "Player Hit_Stun")
      (`|PlayMontage` (`self.Mesh`) "/Game/_Resource/Character/Player/Animation/abn_stun_1_Montage.abn_stun_1_Montage"
        (:`then`
          ; 캐릭터를 노란색으로 깜빡이게 한다
          (`|ExecutionSequence`
            (:`then_0`
              (`MaterialInstanceDynamic.SetVectorParameterValue` (`self.Material_0`) "Tint" (struct :`R` 1.0 :`G` 0.886706 :`A` 1.0)))
            (:`then_1`
              (`MaterialInstanceDynamic.SetVectorParameterValue` (`self.Material_1`) "Tint" (struct :`R` 1.0 :`G` 0.808155 :`A` 1.0))))
          (`KismetSystemLibrary.Delay` 0.15)
          (`|ExecutionSequence`
            (:`then_0`
              (`MaterialInstanceDynamic.SetVectorParameterValue` (`self.Material_0`) "Tint" (struct :`R` 1.0 :`G` 1.0 :`B` 1.0 :`A` 1.0)))
            (:`then_1`
              (`MaterialInstanceDynamic.SetVectorParameterValue` (`self.Material_1`) "Tint" (struct :`R` 1.0 :`G` 1.0 :`B` 1.0 :`A` 1.0)))))))
    (:`NewEnumerator3`
      (`KismetSystemLibrary.PrintString` "Player Hit_Knockback")
      ; 캐릭터를 초록색으로 깜빡이게 한다
      (`|ExecutionSequence`
        (:`then_0`
          (`MaterialInstanceDynamic.SetVectorParameterValue` (`self.Material_0`) "Tint" (struct :`R` 0.197574 :`G` 1.0 :`A` 1.0)))
        (:`then_1`
          (`MaterialInstanceDynamic.SetVectorParameterValue` (`self.Material_1`) "Tint" (struct :`R` 0.376673 :`G` 1.0 :`A` 1.0))))
      (`KismetSystemLibrary.Delay` 0.15)
      (`|ExecutionSequence`
        (:`then_0`
          (`MaterialInstanceDynamic.SetVectorParameterValue` (`self.Material_0`) "Tint" (struct :`R` 1.0 :`G` 1.0 :`B` 1.0 :`A` 1.0)))
        (:`then_1`
          (`MaterialInstanceDynamic.SetVectorParameterValue` (`self.Material_1`) "Tint" (struct :`R` 1.0 :`G` 1.0 :`B` 1.0 :`A` 1.0)))))
    (:`NewEnumerator4`
      (if (`self.canKnockDown`)
        (`KismetSystemLibrary.PrintString` "Player Hit_Knockdown")
        (`|PlayMontage` (`self.Mesh`) "/Game/_Resource/Character/Player/Animation/bound_Montage.bound_Montage"
          (:`then`
            (set `self.canKnockDown` false)
            ; 캐릭터를 파란색으로 깜빡이게 한다
            (`|ExecutionSequence`
              (:`then_0`
                (`MaterialInstanceDynamic.SetVectorParameterValue` (`self.Material_0`) "Tint" (struct :`G` 0.161012 :`B` 1.0 :`A` 1.0)))
              (:`then_1`
                (`MaterialInstanceDynamic.SetVectorParameterValue` (`self.Material_1`) "Tint" (struct :`G` 0.024614 :`B` 1.0 :`A` 1.0))))
            (`KismetSystemLibrary.Delay` 0.15)
            (`|ExecutionSequence`
              (:`then_0`
                (`MaterialInstanceDynamic.SetVectorParameterValue` (`self.Material_0`) "Tint" (struct :`R` 1.0 :`G` 1.0 :`B` 1.0 :`A` 1.0)))
              (:`then_1`
                (`MaterialInstanceDynamic.SetVectorParameterValue` (`self.Material_1`) "Tint" (struct :`R` 1.0 :`G` 1.0 :`B` 1.0 :`A` 1.0)))))
          (:`OnCompleted`
            (set `self.canKnockDown` true)))))))

(event `self.ReceiveAnyDamage`
  (params (Damage :type "Float (single-precision)") (DamageType :type "DamageType Object Reference") (InstigatedBy :type "Controller Object Reference") (DamageCauser :type "Actor Object Reference"))
  (`self.OnTakeDamage` Damage)
  (goto _label))

(event `self.OnDie`
  (`KismetSystemLibrary.PrintString` "애니메이션 추가, 페이드아웃 이펙트, UI ")
  (`KismetSystemLibrary.Delay` 2.0)
  (`self.K2_DestroyActor`))

(event `self.OnKill`)

(event `self.OnRevival`)

(event `Key|Z`
  (params (Key :type "Key Structure"))
  ; Debug
)

(event `Key|X`
  (params (Key :type "Key Structure"))
  ; Debug
)

(event `Key|C`
  (params (Key :type "Key Structure"))
  ; Debug
)

(fn `UserConstructionScript`)