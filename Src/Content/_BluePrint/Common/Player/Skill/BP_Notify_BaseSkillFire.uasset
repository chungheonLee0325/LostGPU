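; BP_Notify_BaseSkillFire is an animation notify that triggers the fire moment of the skill a player character is casting.
; It casts the mesh owner to BP_Character and reads the CurrentCastSkill map on its PlayerSkillController.
; Only when that map holds exactly one entry does it call OnSkillFire on that skill, so the animation controls the timing.
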(fn `GetNotifyName`
  (returns (ReturnValue :type String))
  (return ""))

(fn `Received_Notify`
  (params (MeshComp :type "SkeletalMeshComponent Object Reference") (Animation :type "AnimSequenceBase Object Reference") (EventReference :type "AnimNotifyEventReference Structure (by ref)"))
  (returns (ReturnValue :type Boolean))
  (bind _asbp_character (cast `/Game/_BluePrint/Common/BP_Character` (`ActorComponent.GetOwner` MeshComp)))
  (bind _currentcastskill (`/Game/_BluePrint/Common/Player/Skill/PlayerSkillController.currentCastSkill` (`/Game/_BluePrint/Common/BP_Character.PlayerSkillController` _asbp_character)))
  (if (== (`BlueprintMapLibrary.Map_Length` _currentcastskill) 1)
    (bind _values (`BlueprintMapLibrary.Map_Values` _currentcastskill))
    (`/Game/_BluePrint/Common/Skill/BP_Skill_Base.On_Skill_Fire` (`|GetArrayItem` _values (`KismetArrayLibrary.Array_LastIndex` _values)))
    (return false)))