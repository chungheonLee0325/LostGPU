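; BP_Skill_Space is a player skill, apparently for the Space slot, that extends a parent skill class.
; On cast it runs the parent logic, then turns the player pawn's yaw toward the point under the mouse cursor, found by a Visibility trace.
; Its cooldown override runs the parent calculation, then pushes the values to the skill slot UI through BP_Character's HUD, in code marked as provisional.
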(fn `CalcCoolTime`
  ; CoolTime 가구현 코드!!!! 수정 필요
  (`parent.CalcCoolTime`)
  (bind _asbp_character (cast `/Game/_BluePrint/Common/BP_Character` (`GameplayStatics.GetPlayerPawn` 0)))
  (`/Game/_BluePrint/Common/Widget/HUD_SkiilSlot.SetCoolTimeUI` (`/Game/_BluePrint/Common/Widget/HUD_Player.HUD_SkiilSlot` (`/Game/_BluePrint/Common/Widget/HUD.HUD_Player` (`/Game/_BluePrint/Common/BP_Character.HUD Reference` _asbp_character))) "NewEnumerator10" (`self.CoolTime`) (`self.currentCoolTime`)))

(fn `On_Skill_Cast`
  (returns (Success :type Boolean))
  (bind _returnvalue (`GameplayStatics.GetPlayerPawn` 0))
  (bind (_returnvalue_roll _returnvalue_pitch) (`KismetMathLibrary.BreakRotator` (`Actor.K2_GetActorRotation` _returnvalue)))
  (bind (_returnvalue_roll_2 _returnvalue_pitch_2 _returnvalue_yaw) (`KismetMathLibrary.BreakRotator` (`KismetMathLibrary.FindLookAtRotation` (`Actor.K2_GetActorLocation` _returnvalue) (`.Location` (`GameplayStatics.BreakHitResult` (`PlayerController.GetHitResultUnderCursorByChannel` (`GameplayStatics.GetPlayerController` 0) "TraceTypeQuery1" true))))))
  (bind _success (`parent.On_Skill_Cast`))
  (`Actor.K2_SetActorRotation` _returnvalue (`KismetMathLibrary.MakeRotator` _returnvalue_roll _returnvalue_pitch _returnvalue_yaw) false)
  (return _success))