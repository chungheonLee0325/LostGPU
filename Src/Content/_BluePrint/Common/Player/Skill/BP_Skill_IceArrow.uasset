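; BP_Skill_IceArrow is a player skill Blueprint that, despite its name, casts a counter skill by spawning BP_CounterSkill.
; On OnSkillCast, it turns the player pawn toward the visibility hit under the cursor, using the pawn's own Z so the aim stays level.
; It then stores a point a fixed distance ahead in SkillDir and spawns BP_CounterSkill there with the player's yaw.
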(event `self.On_Skill_Cast`
  (bind _returnvalue (`GameplayStatics.GetPlayerPawn` 0))
  (bind (_returnvalue_x _returnvalue_y _returnvalue_z) (`KismetMathLibrary.BreakVector` (`Actor.K2_GetActorLocation` (`GameplayStatics.GetPlayerPawn` 0))))
  (bind _returnvalue_2 (`Actor.GetTransform` _returnvalue))
  (bind (_bblockinghit _binitialoverlap _time _distance _location) (`GameplayStatics.BreakHitResult` (`PlayerController.GetHitResultUnderCursorByChannel` (`GameplayStatics.GetPlayerController` 0) "TraceTypeQuery1" true)))
  ; 카운터 스킬
  (`Actor.K2_SetActorRotation` _returnvalue (`KismetMathLibrary.FindLookAtRotation` (.location _returnvalue_2) (`KismetMathLibrary.MakeVector` (.x _location) (.y _location) _returnvalue_z)) false)
  (bind _output_get (set `self.SkillDir` (+ (* (`Actor.GetActorForwardVector` _returnvalue) 300.0) (.location _returnvalue_2))))
  (`|SpawnActorFromClass` "/Game/_BluePrint/JJH/BP_CounterSkill.BP_CounterSkill_C" (`KismetMathLibrary.MakeTransform` _output_get (`KismetMathLibrary.MakeRotator` 0.0 0.0 (.yaw (.rotation _returnvalue_2)))) "Undefined" "MultiplyWithRoot" null null))