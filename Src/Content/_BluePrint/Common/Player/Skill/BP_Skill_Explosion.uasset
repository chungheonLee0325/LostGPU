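; Player skill Blueprint, named Explosion, that fires a BP_Element_FireBall toward the mouse cursor.
; On a successful parent cast check, it turns the player toward the cursor hit at the player's height and stores a spawn point ahead and the yaw.
; The skill-fire event spawns the fireball from those stored values.
; The cooldown override pushes timing to a fixed HUD skill slot and is marked as provisional code.
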(event `self.On_Skill_Fire`
  (`|SpawnActorFromClass` "/Game/_BluePrint/Common/Player/Skill/BP_Element_FireBall.BP_Element_FireBall_C" (`KismetMathLibrary.MakeTransform` (`self.SkillDir`) (`KismetMathLibrary.MakeRotator` 0.0 0.0 (`self.Return Value Rotation Z (Yaw)`))) "Undefined" "MultiplyWithRoot" null 1100.0 null))

(fn `CalcCoolTime`
  ; CoolTime 가구현 코드!!!! 수정 필요
  (`parent.CalcCoolTime`)
  (bind _asbp_character (cast `/Game/_BluePrint/Common/BP_Character` (`GameplayStatics.GetPlayerPawn` 0)))
  (`/Game/_BluePrint/Common/Widget/HUD_SkiilSlot.SetCoolTimeUI` (`/Game/_BluePrint/Common/Widget/HUD_Player.HUD_SkiilSlot` (`/Game/_BluePrint/Common/Widget/HUD.HUD_Player` (`/Game/_BluePrint/Common/BP_Character.HUD Reference` _asbp_character))) "NewEnumerator0" (`self.CoolTime`) (`self.currentCoolTime`)))

(fn `On_Skill_Cast`
  (returns (Success :type Boolean))
  (bind _returnvalue (`GameplayStatics.GetPlayerPawn` 0))
  (bind (_returnvalue_x _returnvalue_y _returnvalue_z) (`KismetMathLibrary.BreakVector` (`Actor.K2_GetActorLocation` (`GameplayStatics.GetPlayerPawn` 0))))
  (bind _returnvalue_2 (`Actor.GetTransform` _returnvalue))
  (bind (_bblockinghit _binitialoverlap _time _distance _location) (`GameplayStatics.BreakHitResult` (`PlayerController.GetHitResultUnderCursorByChannel` (`GameplayStatics.GetPlayerController` 0) "TraceTypeQuery1" true)))
  (bind _success (`parent.On_Skill_Cast`))
  ; 카운터 스킬
  (if _success
    (`Actor.K2_SetActorRotation` _returnvalue (`KismetMathLibrary.FindLookAtRotation` (.location _returnvalue_2) (`KismetMathLibrary.MakeVector` (.x _location) (.y _location) _returnvalue_z)) false)
    (set `self.SkillDir` (+ (* (`Actor.GetActorForwardVector` _returnvalue) 100.0) (.location _returnvalue_2)))
    (set `self.Return Value Rotation Z (Yaw)` (.yaw (.rotation _returnvalue_2))))
  (return _success))