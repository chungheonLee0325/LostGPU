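; BP_Element_FireBall is a fireball element skill projectile for the player, extending a parent class's BeginPlay and Hit behavior.
; It plays a 2D explosion launch sound on spawn.
; On hit, it plays an impact sound, sends a destruct damage message to the struck actor and applies its Damage value.
; It also triggers a world camera shake at the hit location that falls off with distance.
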(event `self.ReceiveBeginPlay`
  (`parent.ReceiveBeginPlay`)
  (`GameplayStatics.PlaySound2D` "/Game/_Resource/Sound/Player_Skill/익스플로전_발사.익스플로전_발사" 1.0 1.0 0.0 null null))

(event `self.ReceiveHit`
  (params (MyComp :type "PrimitiveComponent Object Reference") (Other :type "Actor Object Reference") (OtherComp :type "PrimitiveComponent Object Reference") (bSelfMoved :type Boolean) (HitLocation :type "Vector Structure") (HitNormal :type "Vector Structure") (NormalImpulse :type "Vector Structure") (Hit :type "HitResult Structure (by ref)"))
  (`parent.ReceiveHit` MyComp Other OtherComp bSelfMoved HitLocation HitNormal NormalImpulse Hit)
  (`GameplayStatics.PlaySound2D` "/Game/_Resource/Sound/Player_Skill/익스플로전_히트.익스플로전_히트" 1.0 1.0 0.0 null null)
  (message `/Game/_BluePrint/Common/Interface/IDestructibleActor.ApplyDestructDamage` Other 1)
  (`GameplayStatics.ApplyDamage` Other (`self.Damage`))
  (`GameplayStatics.PlayWorldCameraShake` "/Game/_BluePrint/Common/CameraShake/BP_CS_L.BP_CS_L_C" HitLocation 1000.0 3000.0))

(fn `UserConstructionScript`
  (`parent.UserConstructionScript`))