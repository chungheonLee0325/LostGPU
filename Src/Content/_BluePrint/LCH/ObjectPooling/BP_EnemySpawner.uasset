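; BP_EnemySpawner is a timed spawner that requests objects from a BP_ObjectPool, presumably enemies.
; On BeginPlay, CreateEnemy only picks a random interval between MinRTime and MaxRTime, despite its name.
; Tick accumulates time and, each time the interval elapses, resets the timer and calls GetObject on the pool.
; The interval is never re-randomized, so each spawner keeps a fixed rhythm.
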(event `self.ReceiveBeginPlay`
  (`self.CreateEnemy`))

(event `self.ReceiveTick`
  (params (DeltaSeconds :type "Float (single-precision)"))
  (bind _output_get (set `self.CurrentTime` (+ DeltaSeconds (`self.CurrentTime`))))
  (if (> _output_get (`self.CreateTime`))
    (set `self.CurrentTime` 0.0)
    (bind _asbp_object_pool (cast `/Game/_BluePrint/LCH/ObjectPooling/BP_ObjectPool` (`self.ObjectPool`)))
    (`/Game/_BluePrint/LCH/ObjectPooling/BP_ObjectPool.GetObject` _asbp_object_pool)))

(fn `CreateEnemy`
  (set `self.CreateTime` (`KismetMathLibrary.RandomFloatInRange` (`self.MinRTime`) (`self.MaxRTime`))))

(fn `UserConstructionScript`)