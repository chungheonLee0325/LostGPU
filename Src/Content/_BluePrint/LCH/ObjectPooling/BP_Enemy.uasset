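; BP_Enemy is a pooled enemy that moves in a straight line with a swept move each tick.
; On BeginPlay and each activation, FindDirection picks world up or, by TargetingProbability, the normalized player-to-enemy vector (pointing away from the player as written).
; Box overlap recycles the enemy through DestroyedRObject, along with the other actor if it is a BP_RecycleObject.
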(event `self.ReceiveBeginPlay`
  (set `self.Target` (`GameplayStatics.GetPlayerPawn` 0))
  (`self.FindDirection`))

(event `self.ReceiveActorBeginOverlap`
  (params (OtherActor :type "Actor Object Reference")))

(event `self.ReceiveTick`
  (params (DeltaSeconds :type "Float (single-precision)"))
  (`self.K2_SetActorLocation` (+ (* (* (`self.direction`) (`self.Speed`)) DeltaSeconds) (`self.K2_GetActorLocation`)) true))

(event `self.Box.OnComponentBeginOverlap`
  (params (OverlappedComponent :type "PrimitiveComponent Object Reference") (OtherActor :type "Actor Object Reference") (OtherComp :type "PrimitiveComponent Object Reference") (OtherBodyIndex :type Integer) (bFromSweep :type Boolean) (SweepResult :type "HitResult Structure (by ref)"))
  (`self.Destroyed_RObject`)
  (bind _asbp_recycle_object (cast `/Game/_BluePrint/LCH/ObjectPooling/BP_RecycleObject` OtherActor))
  (`self.Destroyed_RObject` _asbp_recycle_object))

(fn `Destroyed_RObject`
  (`parent.Destroyed_RObject`))

(fn `FindDirection`
  ; 단순 up
  (set `self.direction` (`KismetMathLibrary.GetUpVector` (struct)))
  (if (not (`KismetSystemLibrary.IsValid` (`self.Target`)))
    (set `self.Target` (`GameplayStatics.GetPlayerPawn` 0)))
  ; 확률로 추적 or 단순up
  (if (>= (`self.TargetingProbability`) (`KismetMathLibrary.RandomFloat`))
    (bind _output_get (set `self.TargetLocation` (`self.K2_GetActorLocation` (`self.Target`))))
    (set `self.direction` (`KismetMathLibrary.Normal` (- (`self.K2_GetActorLocation`) _output_get)))))

(fn `SetActive`
  (params (_bool :type Boolean))
  (`parent.SetActive` _bool)
  (if _bool
    (`self.FindDirection`)))

(fn `UserConstructionScript`)