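; BP_ObjectPool is an actor that pre-spawns and reuses BP_RecycleObject actors of a configurable class.
; On BeginPlay, CreatePool spawns a batch at its own transform, injects itself into each object and stores it inactive.
; GetObject activates and removes the first entry, spawning another batch when one or none remain.
; RestoreObject appends returned objects to the pool without deactivating them itself.
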(event `self.ReceiveBeginPlay`
  (`self.CreatePool` (`self.objectType`) (`self.poolSize`)))

(fn `CreatePool`
  (params (objectType :type "Actor Class Reference") (poolSize :type Integer))
  (if (!= objectType "/Script/FractureEditor.FractureToolSelectNone")
    (bind _output_get (set `self.objectType` objectType)))
  (if (!= poolSize 0)
    (bind _output_get_2 (set `self.poolSize` poolSize)))
  (for _ (range (+ _output_get_2 1))
    (bind _returnvalue (`|SpawnActorFromClass` _output_get (`self.GetTransform`) "Undefined" "MultiplyWithRoot" null null))
    (bind _asbp_recycle_object (cast `/Game/_BluePrint/LCH/ObjectPooling/BP_RecycleObject` _returnvalue))
    (`/Game/_BluePrint/LCH/ObjectPooling/BP_RecycleObject.Injection_Factory` _asbp_recycle_object self)
    (`KismetArrayLibrary.Array_Add` (`self.pool`) _asbp_recycle_object)
    (`/Game/_BluePrint/LCH/ObjectPooling/BP_RecycleObject.SetActive` _asbp_recycle_object false)))

(fn `GetObject`
  (returns (NewParam :type "Actor Object Reference"))
  (locals (result :type "Actor Object Reference"))
  (bind _pool (`self.pool`))
  (if (<= (`KismetArrayLibrary.Array_Length` _pool) 1)
    (`self.CreatePool` (`self.objectType`) (`self.poolSize`)))
  (bind _output_get (set `local.result` (`|GetArrayItem` _pool)))
  (`KismetArrayLibrary.Array_Remove` _pool)
  (bind _asbp_recycle_object (cast `/Game/_BluePrint/LCH/ObjectPooling/BP_RecycleObject` _output_get))
  (`/Game/_BluePrint/LCH/ObjectPooling/BP_RecycleObject.SetActive` _asbp_recycle_object true)
  (return _output_get))

(fn `RestoreObject`
  (params (recycleObject :type "Actor Object Reference"))
  (bind _asbp_recycle_object (cast `/Game/_BluePrint/LCH/ObjectPooling/BP_RecycleObject` recycleObject)
    (:`then`
      (`KismetArrayLibrary.Array_Add` (`self.pool`) _asbp_recycle_object))
    (:`CastFailed`
      (`KismetSystemLibrary.PrintString` "Hello"))))

(fn `UserConstructionScript`)