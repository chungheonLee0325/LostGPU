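; BP_RecycleObject is an actor that can be recycled through a BP_ObjectPool instead of being destroyed.
; The owning pool is injected and stored as its factory.
; When released, it restores itself to that pool and deactivates, or destroys itself if the pool cast fails.
; Activation toggles visibility, tick and collision together.
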(event `self.ReceiveBeginPlay`)

(fn `Destroyed_RObject`
  (bind _asbp_object_pool (cast `/Game/_BluePrint/LCH/ObjectPooling/BP_ObjectPool` (`self.OwnFactory`))
    (:`then`
      (`/Game/_BluePrint/LCH/ObjectPooling/BP_ObjectPool.RestoreObject` _asbp_object_pool self)
      (`self.SetActive` false))
    (:`CastFailed`
      (`self.K2_DestroyActor`))))

(fn `Injection_Factory`
  (params (pool :type "Actor Object Reference"))
  (set `self.OwnFactory` pool))

(fn `SetActive`
  (params (_bool :type Boolean))
  (`self.SetActorHiddenInGame` (not _bool))
  (`self.SetActorTickEnabled` _bool)
  (`self.SetActorEnableCollision` _bool))

(fn `UserConstructionScript`)