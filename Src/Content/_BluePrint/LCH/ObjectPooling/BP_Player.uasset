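; Player actor that moves along input and fires bullets taken from an object pool.
; Horizontal and Vertical axis events share one Direction assignment on Y and Z, which Tick normalizes and scales by Speed for a swept move.
; Fire gets an object from the BulletLauncher pool, moves it to FirePosition and adds an audio component to it.
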(event `self.ReceiveBeginPlay`)

(event `self.ReceiveTick`
  (params (DeltaSeconds :type "Float (single-precision)"))
  (`self.K2_SetActorLocation` self (+ (* DeltaSeconds (* (`self.Speed`) (`KismetMathLibrary.Normal` (stale `InputAxis|Horizontal` _output_get)))) (`self.K2_GetActorLocation` self)) true false))

(event `InputAxis|Horizontal`
  (params (AxisValue :type "Float (single-precision)"))
  (bind _output_get (set `self.Direction` (`KismetMathLibrary.MakeVector` 0.0 AxisValue (stale `InputAxis|Vertical` AxisValue)) :!label _label)))

(event `InputAxis|Vertical`
  (params (AxisValue :type "Float (single-precision)"))
  (goto _label))

(event `InputAction|Fire`
  (params (Key :type "Key Structure"))
  (:`Pressed`
    (bind _asbp_object_pool (cast `/Game/_BluePrint/LCH/ObjectPooling/BP_ObjectPool` (`self.BulletLauncher`)))
    (bind _newparam (`/Game/_BluePrint/LCH/ObjectPooling/BP_ObjectPool.GetObject` _asbp_object_pool))
    (bind _asbp_recycle_object (cast `/Game/_BluePrint/LCH/ObjectPooling/BP_RecycleObject` _newparam))
    (`self.K2_SetActorLocation` _asbp_recycle_object (`SceneComponent.K2_GetComponentLocation` (`self.FirePosition`)) true false)
    (`AddComponent|NODE_AddAudioComponent-1` :`self` _asbp_recycle_object)))

(fn `Plus`
  (params (num1 :type Integer) (num2 :type Integer))
  (returns (result :type Integer))
  (set `self.Number2` num2)
  (return (+ num1 num2)))

(fn `UserConstructionScript`)