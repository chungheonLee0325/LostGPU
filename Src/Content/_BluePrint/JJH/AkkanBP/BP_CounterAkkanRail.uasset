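; Rail effect actor for Akkan's counter pattern that shows a fill growing along a rail.
; Tick runs the Filling timeline, which widens FillLail on X while scrolling the rail's dynamic material through its V_Offset parameter.
; The actor destroys itself when the fill reaches full scale, or earlier if the BP_CounterAkkan found in the level reports a counter hit.
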(event `self.ReceiveBeginPlay`
  (bind _returnvalue (`PrimitiveComponent.CreateDynamicMaterialInstance` (`self.Lail`) 0 null "None"))
  (bind _output_get (set `self.LailMat` _returnvalue))
  (bind _returnvalue_2 (`MaterialInstanceDynamic.K2_GetScalarParameterValue` _output_get "V_Offset"))
  (set `self.LailMat_VOffset` _returnvalue_2))

(event `self.ReceiveTick`
  (params (DeltaSeconds :type "Float (single-precision)"))
  (bind (_returnvalue_x _returnvalue_y _returnvalue_z) (`KismetMathLibrary.BreakVector` (`SceneComponent.K2_GetComponentScale` (`self.FillLail`))))
  (bind (_direction _xsize) (`Timeline|Filling` :`NewTime` DeltaSeconds)
    (:`Update`
      (bind _output_get (set `self.LailMat_VOffset` (+ (* DeltaSeconds 0.5) (`self.LailMat_VOffset`))))
      (`MaterialInstanceDynamic.SetScalarParameterValue` (`self.LailMat`) "V_Offset" _output_get)
      (`SceneComponent.SetWorldScale3D` (`self.FillLail`) (`KismetMathLibrary.MakeVector` _xsize _returnvalue_y _returnvalue_z))
      (if (>= _returnvalue_x 18.0)
        ; 카운터 아칸을 불러오고 없으면 레일 파괴
        (`self.K2_DestroyActor` :!label _label)
        (else
          (bind _returnvalue (`GameplayStatics.GetActorOfClass` "/Game/_BluePrint/JJH/AkkanBP/BP_CounterAkkan.BP_CounterAkkan_C"))
          (`/Engine/EditorBlueprintResources/StandardMacros.IsValid` _returnvalue
            (:`Is Valid`
              (if (`/Game/_BluePrint/JJH/AkkanBP/BP_CounterAkkan.IsHittedCounter` _returnvalue)
                (goto _label)))))))))

(fn `UserConstructionScript`)