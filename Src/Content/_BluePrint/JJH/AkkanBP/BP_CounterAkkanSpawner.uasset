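; Spawner attached to the Akkan boss that periodically spawns counter mobs and lasers after the boss cinematic ends, while Akkan is alive.
; BeginPlay caches eight points on a circle sized by the SpawnArea sphere.
; Tick runs two timers, each held at zero while its actor exists, with counter spawns taking priority.
; Lasers randomly take one of two orientations, recording alternating point indices that center-facing counter mobs avoid.
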(event `self.ReceiveBeginPlay`
  (`self.MakeSpawnLocation`))

(event `self.ReceiveTick`
  (params (DeltaSeconds :type "Float (single-precision)"))
  (bind _asbp_akkan (cast `/Game/_BluePrint/JJH/AkkanBP/BP_Akkan` (`self.GetAttachParentActor`)))
  (bind _output_get (set `self.Akkan` _asbp_akkan))
  (if (`/Game/_BluePrint/JJH/AkkanBP/BP_Akkan.Akkan_isCinemacinePlayEnd` _output_get)
    (if (not (`/Game/_BluePrint/Common/AreaObject.IsDead` _output_get))
      ; 시간이 흐른다
      (set `self.SpawnCurrentTime` (+ (`self.SpawnCurrentTime`) DeltaSeconds))
      ;; 카운터 몹 존재하면 스폰시간 초기화
      (bind _returnvalue (`GameplayStatics.GetActorOfClass` "/Game/_BluePrint/JJH/AkkanBP/BP_CounterAkkan.BP_CounterAkkan_C"))
      (`/Engine/EditorBlueprintResources/StandardMacros.IsValid` _returnvalue
        (:`Is Valid`
          (set `self.SpawnCurrentTime` 0.0))
        (:`Is Not Valid`
          _))
      (set `self.LaserCurrentTime` (+ DeltaSeconds (`self.LaserCurrentTime`)))
      (bind _returnvalue_2 (`GameplayStatics.GetActorOfClass` "/Game/_BluePrint/JJH/AkkanSkillBP/BP_AkkanLaser.BP_AkkanLaser_C"))
      (`/Engine/EditorBlueprintResources/StandardMacros.IsValid` _returnvalue_2
        (:`Is Valid`
          (set `self.LaserCurrentTime` 0.0))
        (:`Is Not Valid`
          _))
      ; 스폰시간 체크
      (if (<= (`self.SpawnTime`) (`self.SpawnCurrentTime`))
        (`self.SpawnCounterAkkan`)
        (else
          ; 레이저시간 체크
          (if (<= (`self.LaserTime`) (`self.LaserCurrentTime`))
            (`self.MakeLaserLocationIndices`)
            (if (== (`self.RandomArrayIdx`) 0)
              (set `self.LaserRotation` (struct :`Yaw` 45.0))
              (else
                (set `self.LaserRotation` (struct))))
            (`|SpawnActorFromClass` "/Game/_BluePrint/JJH/AkkanSkillBP/BP_AkkanLaser.BP_AkkanLaser_C" (`KismetMathLibrary.MakeTransform` (`SceneComponent.K2_GetComponentLocation` (`/Game/_BluePrint/JJH/AkkanBP/BP_Akkan.CreateSkillPivot` (`self.Akkan`))) (`self.LaserRotation`)) "Undefined" "MultiplyWithRoot" null null)))))))

(fn `MakeLaserLocationIndices`
  (bind _returnvalue (`GameplayStatics.GetActorOfClass` "/Game/_BluePrint/JJH/AkkanSkillBP/BP_AkkanLaser.BP_AkkanLaser_C"))
  (`/Engine/EditorBlueprintResources/StandardMacros.IsValid` _returnvalue
    (:`Is Not Valid`
      ; idx array 초기화 후, 0~1의 랜덤 값 생성
      (`KismetArrayLibrary.Array_Clear` (`self.LaserLocationIdx`))
      (bind _output_get (set `self.RandomArrayIdx` (`KismetMathLibrary.RandomIntegerInRange` 0 1)))
      (if (== _output_get 0)
        ; (0,2,4,6) 좌표 반환
        (for _index (range 4)
          (`KismetArrayLibrary.Array_Add` (`self.LaserLocationIdx`) (+ (* _index 2) (`self.RandomArrayIdx`))))
        (else
          ; (1,3,5,7) 좌표 반환
          (for _index_2 (range 4)
            (`KismetArrayLibrary.Array_Add` (`self.LaserLocationIdx`) (+ (* _index_2 2) (`self.RandomArrayIdx`)))))))))

(fn `MakeSpawnLocation`
  (for _index (range 1 9)
    (bind _returnvalue (`KismetMathLibrary.DegreesToRadians` (* _index (`self.RangeAngle`))))
    ; x = cosΘ * radius
    (bind _output_get (set `self.RandomX` (* (`KismetMathLibrary.Cos` _returnvalue) (`SphereComponent.GetScaledSphereRadius` (`self.SpawnArea`)))))
    ; y = sinΘ * radius
    (bind _output_get_2 (set `self.RandomY` (* (`KismetMathLibrary.Sin` _returnvalue) (`SphereComponent.GetScaledSphereRadius` (`self.SpawnArea`)))))
    (bind _output_get_3 (set `self.RandomLoc` (`KismetMathLibrary.MakeVector` _output_get _output_get_2)))
    (`KismetArrayLibrary.Array_Add` (`self.SpawnLocations`) (+ _output_get_3 (`self.K2_GetActorLocation`)))))

(fn `SpawnCounterAkkan`
  (bind _output (`|GetArrayItem` (`self.SpawnLocations`) (`self.RandomLocIdx`)))
  (bind (_returnvalue_roll _returnvalue_pitch _returnvalue_yaw) (`KismetMathLibrary.BreakRotator` (`KismetMathLibrary.FindLookAtRotation` _output (`self.K2_GetActorLocation`))))
  (if (`KismetArrayLibrary.Array_IsEmpty` (`self.LaserLocationIdx`))
    ; 레이저 위치이면 다시 random int 생성
    ;; 레이저 존재 하지 않을 때
    (set `self.RandomLocIdx` (`KismetMathLibrary.RandomIntegerInRange` 0 7))
    (else
      ;; 레이저가 존재 할 때
      (while (`KismetArrayLibrary.Array_Contains` (`self.LaserLocationIdx`) (stale _output_get))
        (bind _output_get (set `self.RandomLocIdx` (`KismetMathLibrary.RandomIntegerInRange` 0 7))))))
  ; 해당 위치로 카운터 몹 스폰
  (`|SpawnActorFromClass` "/Game/_BluePrint/JJH/AkkanBP/BP_CounterAkkan.BP_CounterAkkan_C" (`KismetMathLibrary.MakeTransform` _output (`KismetMathLibrary.MakeRotator` 0.0 0.0 _returnvalue_yaw) (0.4 0.4 0.4)) "Undefined" "MultiplyWithRoot" null null))

(fn `UserConstructionScript`)