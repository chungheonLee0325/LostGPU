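; BP_Akkan is a boss that the player must defeat before a time limit kills them.
; Tick runs the phases: material parameter collection visibility ramp, level sequence cinematic, then timed BP_AkkanSkill spawns, held back while one exists.
; Fireball hits deplete DestroyStack; death swaps weapon visibility, reverses the ramp after the montage and triggers GameWin after a delay.
; Tick also pins the actor's location to avoid animation-driven physics bugs.
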(event `SetWeaponVisibility`
  (bind _isweaponhidden (`self.isWeaponHidden`))
  (bind _isstaffhidden (`self.isStaffHidden`))
  (`|ExecutionSequence`
    (:`then_0`
      (`SceneComponent.SetHiddenInGame` (`self.scythe_v1`) _isweaponhidden false))
    (:`then_1`
      (`SceneComponent.SetHiddenInGame` (`self.staff_v2`) _isweaponhidden false))
    (:`then_2`
      (`SceneComponent.SetHiddenInGame` (`self.staff_v3`) _isstaffhidden false))
    (:`then_3`
      (`SceneComponent.SetHiddenInGame` (`self.crosshair`) _isstaffhidden false))))

(event `CallEndEvt`
  ; 종료 연출
  (bind _output_get (set `self.VisibleValue` (+ (`self.VisibleValue`) (* (`self.DieSpeed`) (stale `self.ReceiveTick` DeltaSeconds)))))
  (if (< _output_get 4.0)
    (`KismetMaterialLibrary.SetScalarParameterValue` "/Game/_Resource/Character/Boss/Akkan/AkkanModel/Material/M_Akkan_Param.M_Akkan_Param" "Boss_VisibleValue" (`self.VisibleValue`))
    (else
      (`KismetMaterialLibrary.SetScalarParameterValue` "/Game/_Resource/Character/Boss/Akkan/AkkanModel/Material/M_Akkan_Param.M_Akkan_Param" "Boss_VisibleValue" 4.0))))

(event `Play Akkan Cinematic`
  (bind _outactor (`LevelSequencePlayer.CreateLevelSequencePlayer` "/Game/_Resource/Character/Boss/Akkan/AkkanCinemachine/test.test"))
  (`MovieSceneSequencePlayer.Play` (`LevelSequenceActor.SequencePlayer` _outactor))
  (set `self.Akkan_isCinemachinePlay` true))

(event `self.ReceiveBeginPlay`
  (`parent.ReceiveBeginPlay`)
  (bind _asbp_character (cast `/Game/_BluePrint/Common/BP_Character` (`GameplayStatics.GetPlayerPawn` 0)))
  (set `self.Player` _asbp_character)
  (bind _returnvalue (`KismetMaterialLibrary.GetScalarParameterValue` "/Game/_Resource/Character/Boss/Akkan/AkkanModel/Material/M_Akkan_Param.M_Akkan_Param" "Boss_VisibleValue"))
  (set `self.VisibleValue` _returnvalue)
  ; 애니메이션으로 인한 물리버그 방지 좌표저장
  (set `self.CurrentLoc` (`self.K2_GetActorLocation`)))

(event `CallStartEvt`
  ; 시작 연출
  (bind _output_get (set `self.VisibleValue` (- (`self.VisibleValue`) (* (`self.DieSpeed`) (stale `self.ReceiveTick` DeltaSeconds)))))
  (if (> _output_get -2.0)
    (`KismetMaterialLibrary.SetScalarParameterValue` "/Game/_Resource/Character/Boss/Akkan/AkkanModel/Material/M_Akkan_Param.M_Akkan_Param" "Boss_VisibleValue" (`self.VisibleValue`))
    (else
      (`KismetMaterialLibrary.SetScalarParameterValue` "/Game/_Resource/Character/Boss/Akkan/AkkanModel/Material/M_Akkan_Param.M_Akkan_Param" "Boss_VisibleValue" -2.0)
      (`|ExecutionSequence`
        (:`then_0`
          (set `self.isWeaponHidden` true))
        (:`then_1`
          (set `self.isStaffHidden` false)
          (`self.SetWeaponVisibility`))
        (:`then_2`
          (set `self.Akkan_isStart` true))))))

(event `Check Cinematic End`
  (bind _sequenceplayer (`LevelSequenceActor.SequencePlayer` (stale `Play Akkan Cinematic` _outactor)))
  (if (>= (`TimeManagementBlueprintLibrary.Conv_QualifiedFrameTimeToSeconds` (`MovieSceneSequencePlayer.GetCurrentTime` _sequenceplayer)) (`TimeManagementBlueprintLibrary.Conv_QualifiedFrameTimeToSeconds` (`MovieSceneSequencePlayer.GetEndTime` _sequenceplayer)))
    (set `self.Akkan_isCinemacinePlayEnd` true)))

(event `self.ReceiveTick`
  (params (DeltaSeconds :type "Float (single-precision)"))
  ; 애니메이션으로 인한 충돌 방지
  (`self.K2_SetActorLocation` (`self.CurrentLoc`))
  ; 종료 시간
  (bind _output_get (set `self.CurrentTime` (+ DeltaSeconds (`self.CurrentTime`))))
  (if (< _output_get (`self.PatternEndTime`))
    (if (`self.Akkan_isStart`)
      (if (`self.Akkan_isCinemachinePlay`)
        (if (`self.Akkan_isCinemacinePlayEnd`)
          (if (`self.IsDead`)
            (if (`self.IsMontageEnd`)
              (`self.CallEndEvt`))
            (else
              (bind _output_get_2 (set `self.SkillCurrentTime` (+ DeltaSeconds (`self.SkillCurrentTime`))))
              (if (> _output_get_2 (`self.SkillCreateTime`))
                (set `self.SkillCurrentTime` 0.0)
                (bind _output_get_3 (set `self.AkkanSkillDir` (`SceneComponent.K2_GetComponentLocation` (`self.CreateSkillPivot`))))
                (`|SpawnActorFromClass` "/Game/_BluePrint/JJH/AkkanSkillBP/BP_AkkanSkill.BP_AkkanSkill_C" (`KismetMathLibrary.MakeTransform` _output_get_3) "Undefined" "MultiplyWithRoot" null null)
                (else
                  (bind _returnvalue (`GameplayStatics.GetActorOfClass` "/Game/_BluePrint/JJH/AkkanSkillBP/BP_AkkanSkill.BP_AkkanSkill_C"))
                  (`/Engine/EditorBlueprintResources/StandardMacros.IsValid` _returnvalue
                    (:`Is Valid`
                      (set `self.SkillCurrentTime` 0.0)))))))
          (else
            (`self.Check Cinematic End`)))
        (else
          (`self.Play Akkan Cinematic`)))
      (else
        (`self.CallStartEvt`)))
    (else
      (`self.OnDie` (`self.Player`)))))

(event `self.HitBox.OnComponentBeginOverlap`
  (params (OverlappedComponent :type "PrimitiveComponent Object Reference") (OtherActor :type "Actor Object Reference") (OtherComp :type "PrimitiveComponent Object Reference") (OtherBodyIndex :type Integer) (bFromSweep :type Boolean) (SweepResult :type "HitResult Structure (by ref)"))
  (`self.Akkan_DestoryEvt`))

(event `self.OnDie`
  (set `self.Animations_Dead` "/Game/_Resource/Character/Boss/Akkan/AkkanAnimation/Akkan_DieMontage.Akkan_DieMontage")
  (`|ExecutionSequence`
    (:`then_0`
      (set `self.isWeaponHidden` false))
    (:`then_1`
      (set `self.isStaffHidden` true)
      (`self.SetWeaponVisibility`)
      (`parent.OnDie`)
      (`KismetSystemLibrary.Delay` 8.5)
      (`/Game/_BluePrint/Common/Widget/HUD.GameWin` (`/Game/_BluePrint/Common/BP_Character.HUD Reference` (`self.Player`)))
      (`self.K2_DestroyActor`))))

(event `Akkan_DestoryEvt`
  ; 파괴 스킬 히트 및 파괴 스택 처리 구간
  (if (< (`self.DestroyStack`) 0)
    (`self.OnDie`)))

(event `self.HitBox.OnComponentHit`
  (params (HitComponent :type "PrimitiveComponent Object Reference") (OtherActor :type "Actor Object Reference") (OtherComp :type "PrimitiveComponent Object Reference") (NormalImpulse :type "Vector Structure") (Hit :type "HitResult Structure (by ref)"))
  (cast `/Game/_BluePrint/Common/Player/Skill/BP_Element_FireBall` OtherActor)
  (set `self.DestroyStack` (- (`self.DestroyStack`) 1))
  (`self.Akkan_DestoryEvt`))

(fn `UserConstructionScript`)