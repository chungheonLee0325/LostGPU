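; BP_CounterAkkan is a spawned Akkan that the player can counter, or that charges forward and hinders them.
; BeginPlay spawns a path rail, then Tick timers trigger the counter effect, forward movement and lifetime destruction.
; Overlapping BP_Element_Cyclone marks it countered, halting movement and dissolving it through a Material Parameter Collection scalar before destruction.
; Otherwise, while moving, it damages an overlapping player once and applies a status effect.
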(event `CallDieEvt`
  ; 사망 시 , Dissolve되도록 머테리얼 설정
  (bind _output_get (set `self.VisableValue` (+ (`self.VisableValue`) (* (stale `self.ReceiveTick` DeltaSeconds) (`self.DieSpeed`)))))
  (if (< _output_get 4.0)
    (`KismetMaterialLibrary.SetScalarParameterValue` "/Game/_Resource/Character/Boss/Akkan/AkkanModel/Material/M_Akkan_Param.M_Akkan_Param" "Counter_VisableValue" (`self.VisableValue`))
    (else
      (`KismetMaterialLibrary.SetScalarParameterValue` "/Game/_Resource/Character/Boss/Akkan/AkkanModel/Material/M_Akkan_Param.M_Akkan_Param" "Counter_VisableValue" -2.0)
      (`self.K2_DestroyActor`))))

(event `self.ReceiveTick`
  (params (DeltaSeconds :type "Float (single-precision)"))
  ; 시간이 흐른다
  (bind _output_get (set `self.EntireCurrentTime` (+ DeltaSeconds (`self.EntireCurrentTime`))))
  (`self.MakeCounterEffect` _output_get)
  ; 카운터를 성공하면 이동하지 않고 삭제, 실패하면 이동
  (if (`self.IsHittedCounter`)
    ; 사망 시 , Dissolve되도록 머테리얼 설정
    (`self.CallDieEvt`)
    (else
      ; 카운터 칠 시간이 지나면 움직여라
      (if (> _output_get (`self.CounterEndTime`))
        (set `self.MoveStart` true)
        (`self.MoveForward` DeltaSeconds)
        ; 스폰된 카운터 일리아칸 삭제 시간 설정
        (if (> (`self.EntireCurrentTime`) (`self.LifeTime`))
          (`self.K2_DestroyActor`))))))

(event `self.Collision.OnComponentBeginOverlap`
  (params (OverlappedComponent :type "PrimitiveComponent Object Reference") (OtherActor :type "Actor Object Reference") (OtherComp :type "PrimitiveComponent Object Reference") (OtherBodyIndex :type Integer) (bFromSweep :type Boolean) (SweepResult :type "HitResult Structure (by ref)"))
  ; 카운터 못치면 플레이어 진행 방해
  (bind _asbp_character (cast `/Game/_BluePrint/Common/BP_Character` OtherActor)
    (:`then`
      (if (`self.IsHittedCounter`)
        _
        (elif (`self.MoveStart`)
          (if (not (`self.IsHit`))
            (`GameplayStatics.ApplyDamage` _asbp_character (`self.DmgAmount`))
            (`/Game/_BluePrint/Common/AreaObject.OnStatusEffectApply` _asbp_character "NewEnumerator4" 2.0)
            (set `self.IsHit` true)))))
    (:`CastFailed`
      (cast `/Game/_BluePrint/Common/Player/Skill/BP_Element_Cyclone` OtherActor)
      (set `self.IsHittedCounter` true))))

(event `self.ReceiveBeginPlay`
  ; 시작할 때 지나가는 경로 생성
  (`|SpawnActorFromClass` "/Game/_BluePrint/JJH/AkkanBP/BP_CounterAkkanRail.BP_CounterAkkanRail_C" (`KismetMathLibrary.MakeTransform` (`SceneComponent.K2_GetComponentLocation` (`self.Pivot`)) (`self.K2_GetActorRotation`)) "Undefined" "MultiplyWithRoot" null null)
  (bind _returnvalue (`KismetMaterialLibrary.GetScalarParameterValue` "/Game/_Resource/Character/Boss/Akkan/AkkanModel/Material/M_Akkan_Param.M_Akkan_Param" "Counter_VisableValue"))
  (set `self.VisableValue` _returnvalue))

(fn `MakeCounterEffect`
  (params (CurrentTime :type "Float (double-precision)"))
  ; 카운터 칠 수 있는 시간이 되면 이펙트를 생성한다.
  (if (> CurrentTime (`self.CounterStartTime`))
    (if (not (`self.SpawnCounterEffect`))
      (set `self.SpawnCounterEffect` true)
      (`GameplayStatics.SpawnEmitterAttached` "/Game/StarterContent/Particles/P_Explosion.P_Explosion" (`self.Collision`)))))

(fn `MoveForward`
  (params (DeltaTime :type "Float (single-precision)"))
  ; 앞으로 가라
  (`self.K2_SetActorLocation` (+ (* DeltaTime (* (`self.MoveSpeed`) (`self.GetActorForwardVector`))) (`self.K2_GetActorLocation`)) true))

(fn `UserConstructionScript`)