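; BP_Akkan is an Akkan battle actor that loops an idle animation and periodically spawns BP_AkkanSkill at its CreateSkillPivot.
; Tick accumulates time up to CreateTime, resetting whenever a skill actor exists in the level, so the countdown only advances once none remains.
; Capsule overlap with BP_CounterSkill only prints "Destroyed" when DestroyStack is below one, without changing the stack or destroying anything.
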(event `self.ReceiveBeginPlay`
  (`SkeletalMeshComponent.PlayAnimation` (`self.akkan`) "/Game/_Resource/Character/Boss/Akkan/AkkanAnimation/idle_battle_1.idle_battle_1" true))

(event `self.CapsuleComponent.OnComponentBeginOverlap`
  (params (OverlappedComponent :type "PrimitiveComponent Object Reference") (OtherActor :type "Actor Object Reference") (OtherComp :type "PrimitiveComponent Object Reference") (OtherBodyIndex :type Integer) (bFromSweep :type Boolean) (SweepResult :type "HitResult Structure (by ref)"))
  (cast `/Game/_BluePrint/JJH/BP_CounterSkill` OtherActor)
  (if (< (`self.DestroyStack`) 1)
    (`KismetSystemLibrary.PrintString` "Destroyed")))

(event `self.ReceiveTick`
  (params (DeltaSeconds :type "Float (single-precision)"))
  (bind _output_get (set `self.CurrentTime` (+ DeltaSeconds (`self.CurrentTime`))))
  (if (> _output_get (`self.CreateTime`))
    (set `self.CurrentTime` 0.0)
    (bind _output_get_2 (set `self.AkkanSkillDir` (`SceneComponent.K2_GetComponentLocation` (`self.CreateSkillPivot`))))
    (`|SpawnActorFromClass` "/Game/_BluePrint/JJH/BP_AkkanSkill.BP_AkkanSkill_C" (`KismetMathLibrary.MakeTransform` _output_get_2) "Undefined" "MultiplyWithRoot" null null)
    (else
      (bind _returnvalue (`GameplayStatics.GetActorOfClass` "/Game/_BluePrint/JJH/BP_AkkanSkill.BP_AkkanSkill_C"))
      (`/Engine/EditorBlueprintResources/StandardMacros.IsValid` _returnvalue
        (:`Is Valid`
          (set `self.CurrentTime` 0.0))))))

(fn `UserConstructionScript`)