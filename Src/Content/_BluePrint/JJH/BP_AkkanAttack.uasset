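; BP_AkkanAttack is an attack hitbox actor, apparently for Akkan, that detects contact with the player character.
; A Box overlap with BP_Character prints a debug hit message and destroys the actor, without applying damage.
; Tick accumulates elapsed time and destroys the actor once it exceeds LifeTime.
; An explosion effect at the player's location exists in the graph but is disconnected and never runs.
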(event `self.Box.OnComponentBeginOverlap`
  (params (OverlappedComponent :type "PrimitiveComponent Object Reference") (OtherActor :type "Actor Object Reference") (OtherComp :type "PrimitiveComponent Object Reference") (OtherBodyIndex :type Integer) (bFromSweep :type Boolean) (SweepResult :type "HitResult Structure (by ref)"))
  ; collision에 닿으면 Hit처리
  (bind _asbp_character (cast `/Game/_BluePrint/Common/BP_Character` OtherActor))
  (`/Engine/EditorBlueprintResources/StandardMacros.IsValid` _asbp_character
    (:`Is Valid`
      (`KismetSystemLibrary.PrintString` "Player Hit")
      (`self.K2_DestroyActor` :!label _label))))

(event `self.ReceiveTick`
  (params (DeltaSeconds :type "Float (single-precision)"))
  ; 플레이어가 안맞을때 파괴처리
  (bind _output_get (set `self.CurrentTime` (+ DeltaSeconds (`self.CurrentTime`))))
  (if (> _output_get (`self.LifeTime`))
    (goto _label)))

(fn `UserConstructionScript`)