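; BP_CounterAkkan is a spawned counter Illiakan that the player can counter before it charges forward.
; BeginPlay spawns a BP_CounterAkkanRail at its Pivot to mark the path it will travel.
; Tick runs a timer, attaching an explosion effect when the counter window opens.
; If IsHittedCounter is set after that point it destroys itself; otherwise it later moves forward with a swept move until its destroy time.
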(event `self.ReceiveBeginPlay`
  ; 시작할 때 지나가는 경로 생성
  (`|SpawnActorFromClass` "/Game/_BluePrint/JJH/BP_CounterAkkanRail.BP_CounterAkkanRail_C" (`KismetMathLibrary.MakeTransform` (`SceneComponent.K2_GetComponentLocation` (`self.Pivot`)) (`self.K2_GetActorRotation`)) "Undefined" "MultiplyWithRoot" null null))

(event `self.ReceiveTick`
  (params (DeltaSeconds :type "Float (single-precision)"))
  ; 시간이 흐른다
  (bind _output_get (set `self.CurrentTime` (+ DeltaSeconds (`self.CurrentTime`))))
  ; 카운터 칠 수 있는 시간이 되면 이펙트를 생성한다.
  (if (> _output_get (`self.CounterStartTime`))
    (if (not (`self.SpawnEffect`))
      (set `self.SpawnEffect` true)
      (`GameplayStatics.SpawnEmitterAttached` "/Game/StarterContent/Particles/P_Explosion.P_Explosion" (`self.Collision`)))
    ; 카운터를 성공하면 이동하지 않고 삭제, 실패하면 이동
    (if (`self.IsHittedCounter`)
      (`self.K2_DestroyActor` :!label _label)
      (else
        ; 카운터 칠 시간이 지나고
        (if (> _output_get (`self.CounterEndTime`))
          ; 움직일 수 있는 시간이 되면
          (if (> (`self.CurrentTime`) (`self.MoveStartTime`))
            ; 앞으로가라
            (`self.MoveForward` DeltaSeconds)
            ; 스폰된 카운터 일리아칸 삭제 시간 설정
            (if (> (`self.CurrentTime`) (`self.DestroyTime`))
              (goto _label))))))))

(fn `MoveForward`
  (params (DeltaTime :type "Float (single-precision)"))
  ; 앞으로 가라
  (`self.K2_SetActorLocation` (+ (* DeltaTime (* (`self.Speed`) (`self.GetActorForwardVector`))) (`self.K2_GetActorLocation`)) true))

(fn `UserConstructionScript`)