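; Spawner actor that periodically spawns a BP_CounterAkkan mob and a BP_AkkanLaser attack, allowing one of each at a time.
; On BeginPlay it computes eight points around its SpawnArea sphere.
; Tick runs two timers: before each laser spawns at the center, four alternating indices (even or odd) are recorded as laser slots.
; Counter mobs spawn at a random point outside the last recorded slots, scaled down and facing the center.
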(event `self.ReceiveBeginPlay`
  (`self.MakeSpawnLocation`))

(event `self.ReceiveTick`
  (params (DeltaSeconds :type "Float (single-precision)"))
  ; 시간이 흐른다
  (set `self.SpawnCurrentTime` (+ (`self.SpawnCurrentTime`) DeltaSeconds))
  (set `self.LaserCurrentTime` (+ DeltaSeconds (`self.LaserCurrentTime`)))
  ; 스폰시간 체크
  (if (<= (`self.SpawnTime`) (`self.SpawnCurrentTime`))
    (`self.SpawnCounterAkkan`)
    (set `self.SpawnCurrentTime` 0.0)
    (else
      ; 레이저시간 체크
      (if (<= (`self.LaserTime`) (`self.LaserCurrentTime`))
        ; 레이저 쏘고 있으면 스폰체크시간 초기화
        (bind _returnvalue (`GameplayStatics.GetActorOfClass` "/Game/_BluePrint/JJH/BP_AkkanLaser.BP_AkkanLaser_C"))
        (`/Engine/EditorBlueprintResources/StandardMacros.IsValid` _returnvalue
          (:`Is Valid`
            (set `self.LaserCurrentTime` 0.0))
          (:`Is Not Valid`
            (`self.MakeLaserLocationIndices`)
            (`|SpawnActorFromClass` "/Game/_BluePrint/JJH/BP_AkkanLaser.BP_AkkanLaser_C" (`KismetMathLibrary.MakeTransform` (`self.K2_GetActorLocation`)) "Undefined" "MultiplyWithRoot" null null)
            (set `self.LaserCurrentTime` 0.0)))))))

(fn `MakeLaserLocationIndices`
  (`KismetArrayLibrary.Array_Clear` (`self.LaserLocationIndex`))
  (bind _output_get (set `self.RandomInt` (`KismetMathLibrary.RandomIntegerInRange` 0 1)))
  (if (== 0 _output_get)
    (for _index (range 4)
      (bind _returnvalue (+ (* _index 2) (`self.RandomInt`)))
      (`KismetArrayLibrary.Array_Add` (`self.LaserLocationIndex`) _returnvalue)
      (`KismetSystemLibrary.PrintString` (`KismetStringLibrary.Conv_IntToString` _returnvalue)))
    (else
      (for _index_2 (range 4)
        (bind _returnvalue_2 (+ (* _index_2 2) (`self.RandomInt`)))
        (`KismetArrayLibrary.Array_Add` (`self.LaserLocationIndex`) _returnvalue_2)
        (`KismetSystemLibrary.PrintString` (`KismetStringLibrary.Conv_IntToString` _returnvalue_2))))))

(fn `MakeSpawnLocation`
  (for _index (range 1 9)
    (bind _returnvalue (`KismetMathLibrary.DegreesToRadians` (* _index (`self.RangeAngle`))))
    ; x = cosΘ * radius
    (bind _output_get (set `self.RandomX` (* (`KismetMathLibrary.Cos` _returnvalue) (`SphereComponent.GetScaledSphereRadius` (`self.SpawnArea`)))))
    ; y = sinΘ * radius
    (bind _output_get_2 (set `self.RandomY` (* (`KismetMathLibrary.Sin` _returnvalue) (`SphereComponent.GetScaledSphereRadius` (`self.SpawnArea`)))))
    (bind _output_get_3 (set `self.RandomLoc` (`KismetMathLibrary.MakeVector` _output_get _output_get_2)))
    (`KismetArrayLibrary.Array_Add` (`self.SpawnLocations`) (+ _output_get_3 (`self.K2_GetActorLocation`)))))

(fn `SpawnCounterAkkan`
  (bind _output (`|GetArrayItem` (`self.SpawnLocations`) (`self.RandomInt`)))
  (bind (_returnvalue_roll _returnvalue_pitch _returnvalue_yaw) (`KismetMathLibrary.BreakRotator` (`KismetMathLibrary.FindLookAtRotation` _output (`self.K2_GetActorLocation`))))
  (if (`KismetArrayLibrary.Array_IsEmpty` (`self.LaserLocationIndex`))
    ; 레이저 위치이면 다시 random int 생성
    ;; 레이저 존재 하지 않을 때
    (set `self.RandomInt` (`KismetMathLibrary.RandomIntegerInRange` 0 7))
    (else
      ;; 레이저가 존재 할 때
      (while (`KismetArrayLibrary.Array_Contains` (`self.LaserLocationIndex`) (stale _output_get))
        (bind _output_get (set `self.RandomInt` (`KismetMathLibrary.RandomIntegerInRange` 0 7))))))
  ; 카운터 몹 존재하면 스폰시간 초기화
  (bind _returnvalue (`GameplayStatics.GetActorOfClass` "/Game/_BluePrint/JJH/BP_CounterAkkan.BP_CounterAkkan_C"))
  (`/Engine/EditorBlueprintResources/StandardMacros.IsValid` _returnvalue
    (:`Is Valid`
      (set `self.SpawnCurrentTime` 0.0))
    (:`Is Not Valid`
      ; 해당 위치로 카운터 몹 스폰
      (`|SpawnActorFromClass` "/Game/_BluePrint/JJH/BP_CounterAkkan.BP_CounterAkkan_C" (`KismetMathLibrary.MakeTransform` _output (`KismetMathLibrary.MakeRotator` 0.0 0.0 _returnvalue_yaw) (0.4 0.4 0.4)) "Undefined" "MultiplyWithRoot" null null))))

(fn `UserConstructionScript`)