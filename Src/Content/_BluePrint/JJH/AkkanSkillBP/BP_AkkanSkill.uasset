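; Akkan skill telegraph actor: a fan-shaped range indicator that tracks the player before the attack spawns.
; Tick plays the GettingBigger timeline, whose updates grow the Filling component's Y scale, scroll the Range dynamic material's U_Offset and smoothly rotate the actor toward player 0.
; Once the fill exceeds SkillRange, it spawns BP_AkkanAttack at its own location and rotation, then destroys itself.
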(event `self.ReceiveBeginPlay`
  (bind _returnvalue (`PrimitiveComponent.CreateDynamicMaterialInstance` (`self.Range`) 0 null "None"))
  (bind _output_get (set `self.RangeMat` _returnvalue))
  (bind _returnvalue_2 (`MaterialInstanceDynamic.K2_GetScalarParameterValue` _output_get "U_Offset"))
  (set `self.RangeMat_UOffset` _returnvalue_2))

(event `self.ReceiveTick`
  (params (DeltaSeconds :type "Float (single-precision)"))
  (bind (_returnvalue_location _returnvalue_rotation) (`KismetMathLibrary.BreakTransform` (`self.GetTransform`)))
  (bind _filling (`self.Filling`))
  (bind (_relativescale3d_x _relativescale3d_y _relativescale3d_z) (`KismetMathLibrary.BreakVector` (`SceneComponent.RelativeScale3D` _filling)))
  ; 플레이어를 추적하는 부채꼴 범위가 점점 확장됨
  (bind (_direction _size) (`Timeline|Getting Bigger` :`NewTime` DeltaSeconds)
    (:`Update`
      (bind _output_get (set `self.RangeMat_UOffset` (+ (* DeltaSeconds -0.5) (`self.RangeMat_UOffset`))))
      (`MaterialInstanceDynamic.SetScalarParameterValue` (`self.RangeMat`) "U_Offset" _output_get)
      (`SceneComponent.SetRelativeScale3D` _filling (`KismetMathLibrary.MakeVector` _relativescale3d_x _size _relativescale3d_z))
      (`self.K2_SetActorRotation` (`KismetMathLibrary.RInterpTo` (`self.K2_GetActorRotation`) (`KismetMathLibrary.FindLookAtRotation` (`self.K2_GetActorLocation`) (`self.K2_GetActorLocation` (`GameplayStatics.GetPlayerPawn` 0))) (`GameplayStatics.GetWorldDeltaSeconds`) (`self.LerpSpeed`)))
      ; TimeLine End처리
      (if (> _relativescale3d_y (`self.SkillRange`))
        (`|SpawnActorFromClass` "/Game/_BluePrint/JJH/AkkanSkillBP/BP_AkkanAttack.BP_AkkanAttack_C" (`KismetMathLibrary.MakeTransform` _returnvalue_location _returnvalue_rotation) "Undefined" "MultiplyWithRoot" null null)
        (`self.K2_DestroyActor`)))))

(fn `UserConstructionScript`)