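; BP_AkkanInnerCircle is a filling ground-circle attack for the Akkan skill set that damages the player and triggers the laser.
; A timeline played from Tick grows InnerRadius on a dynamic material while scrolling its U offset.
; When nearly full, it hits once, applying damage and a status effect to an overlapping BP_Character.
; It then finds BP_AkkanLaser, waits briefly, sets LaserStart and destroys itself.
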(event `self.ReceiveBeginPlay`
  (bind _returnvalue (`PrimitiveComponent.CreateDynamicMaterialInstance` (`self.CircleMesh`) 0 "/Game/_BluePrint/JJH/AkkanSkillBP/SkillMaterial/M_AkkanInnerCircle.M_AkkanInnerCircle" "None"))
  (bind _output_get (set `self.CircleMat` _returnvalue))
  (`MaterialInstanceDynamic.K2_GetScalarParameterValue` _output_get "InnerRadius")
  (bind _returnvalue_2 (`MaterialInstanceDynamic.K2_GetScalarParameterValue` _output_get "U_Offset"))
  (set `self.CircleMat_UOffset` _returnvalue_2))

(event `StartLaser`
  (bind _returnvalue (`GameplayStatics.GetActorOfClass` "/Game/_BluePrint/JJH/AkkanSkillBP/BP_AkkanLaser.BP_AkkanLaser_C"))
  (`/Engine/EditorBlueprintResources/StandardMacros.IsValid` _returnvalue
    (:`Is Valid`
      ; 이펙트 추가 부분
      (`KismetSystemLibrary.Delay` 1.0)
      (set `/Game/_BluePrint/JJH/AkkanSkillBP/BP_AkkanLaser.LaserStart` true _returnvalue)
      (`self.K2_DestroyActor`))))

(event `Hit`
  (set `self.isHit` true)
  (if (`self.IsOverlap`)
    (if (`self.CircleHitStart`)
      (bind _asbp_character (cast `/Game/_BluePrint/Common/BP_Character` (`self.CastedPlayer`)))
      (`GameplayStatics.ApplyDamage` _asbp_character (`self.CircleDmgAmount`))
      (`/Game/_BluePrint/Common/AreaObject.OnStatusEffectApply` _asbp_character "NewEnumerator4" 1.0))))

(event `self.ReceiveTick`
  (params (DeltaSeconds :type "Float (single-precision)"))
  (bind _circlemat (`self.CircleMat`))
  (bind (_direction _innercirclesizeup) (`Timeline|Fill` :`NewTime` DeltaSeconds)
    (:`Update`
      (`MaterialInstanceDynamic.SetScalarParameterValue` _circlemat "InnerRadius" _innercirclesizeup)
      (bind _output_get (set `self.CircleMat_UOffset` (+ (`self.CircleMat_UOffset`) (* DeltaSeconds 1.0))))
      (`MaterialInstanceDynamic.SetScalarParameterValue` _circlemat "U_Offset" _output_get)
      (if (> _innercirclesizeup 0.49)
        (set `self.CircleHitStart` true)
        (`|ExecutionSequence`
          (:`then_0`
            (if (not (`self.isHit`))
              (`self.Hit`)))
          (:`then_1`
            (`self.StartLaser`)))))))

(event `self.HitCollision.OnComponentBeginOverlap`
  (params (OverlappedComponent :type "PrimitiveComponent Object Reference") (OtherActor :type "Actor Object Reference") (OtherComp :type "PrimitiveComponent Object Reference") (OtherBodyIndex :type Integer) (bFromSweep :type Boolean) (SweepResult :type "HitResult Structure (by ref)"))
  ; 콜리전 히트 ing 체크
  (set `self.IsOverlap` true)
  (set `self.CastedPlayer` OtherActor))

(event `self.HitCollision.OnComponentEndOverlap`
  (params (OverlappedComponent :type "PrimitiveComponent Object Reference") (OtherActor :type "Actor Object Reference") (OtherComp :type "PrimitiveComponent Object Reference") (OtherBodyIndex :type Integer))
  ; 콜리전 히트 ing 체크
  (set `self.IsOverlap` false))

(fn `UserConstructionScript`)