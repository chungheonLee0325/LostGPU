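; BP_AkkanLaser is an Akkan skill laser that damages and applies a status effect to overlapping characters.
; On BeginPlay it spawns BP_AkkanInnerCircle and keeps the beam mesh hidden until LaserStart is set.
; While active, Tick scrolls the material's U_Offset for animation and destroys the actor after LaserLifeTime.
; After each hit, collision is disabled and a LaserHitTime timer re-enables it, throttling repeat damage.
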(event `self.ReceiveBeginPlay`
  (`|SpawnActorFromClass` "/Game/_BluePrint/JJH/AkkanSkillBP/BP_AkkanInnerCircle.BP_AkkanInnerCircle_C" (`KismetMathLibrary.MakeTransform` (`self.K2_GetActorLocation`) (struct) (`self.InnerCircleSize`)) "Undefined" "MultiplyWithRoot" null null)
  (bind _returnvalue (`PrimitiveComponent.CreateDynamicMaterialInstance` (`self.LaserStaticMesh`) 0 null "None"))
  (bind _output_get (set `self.LaserMat` _returnvalue))
  (bind _returnvalue_2 (`MaterialInstanceDynamic.K2_GetScalarParameterValue` _output_get "U_Offset"))
  (set `self.LaserMat_UOffset` _returnvalue_2)
  (`SceneComponent.SetVisibility` (`self.LaserStaticMesh`) false false)
  (`ActorComponent.Deactivate` (`self.LaserStaticMesh`)))

(event `self.ReceiveTick`
  (params (DeltaSeconds :type "Float (single-precision)"))
  (bind _laserstaticmesh (`self.LaserStaticMesh`))
  (if (`self.LaserStart`)
    (`SceneComponent.SetVisibility` _laserstaticmesh true false)
    (`ActorComponent.SetActive` _laserstaticmesh true false)
    (bind _output_get (set `self.LaserMat_UOffset` (+ (* DeltaSeconds 0.5) (`self.LaserMat_UOffset`))))
    (`MaterialInstanceDynamic.SetScalarParameterValue` (`self.LaserMat`) "U_Offset" _output_get)
    (bind _output_get_2 (set `self.CurrentTime` (+ DeltaSeconds (`self.CurrentTime`))))
    (if (> _output_get_2 (`self.LaserLifeTime`))
      (`self.K2_DestroyActor`))))

(event `CallHitCollision`
  (`PrimitiveComponent.SetCollisionEnabled` (`self.LaserStaticMesh`) "QueryAndPhysics"))

(event `self.LaserStaticMesh.OnComponentBeginOverlap`
  (params (OverlappedComponent :type "PrimitiveComponent Object Reference") (OtherActor :type "Actor Object Reference") (OtherComp :type "PrimitiveComponent Object Reference") (OtherBodyIndex :type Integer) (bFromSweep :type Boolean) (SweepResult :type "HitResult Structure (by ref)"))
  (if (`self.LaserStart`)
    (bind _asbp_character (cast `/Game/_BluePrint/Common/BP_Character` OtherActor))
    (`GameplayStatics.ApplyDamage` _asbp_character (`self.LaserDmgAmount`))
    (`/Game/_BluePrint/Common/AreaObject.OnStatusEffectApply` _asbp_character "NewEnumerator1" 0.7)
    (`PrimitiveComponent.SetCollisionEnabled` (`self.LaserStaticMesh`) "NoCollision")
    (`KismetSystemLibrary.K2_SetTimerDelegate` (delegate `CallHitCollision`) (`self.LaserHitTime`))))

(fn `UserConstructionScript`)